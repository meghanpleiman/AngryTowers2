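; Player controller for the Angry Towers cannon game that routes input to the controlled cannon and shows the points HUD.
; On BeginPlay it creates the number-of-points widget and adds it to the viewport.
; The RaiseCannon axis and Fire action cast the controlled pawn to BP_Cannon and call its matching functions, so the cannon itself handles aiming and firing.
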(event EventBeginPlay
  (bind _returnvalue (UserInterface|CreateWidget "/Game/AngryTowers/WBP_NumberOfPoints.WBP_NumberOfPoints_C" self))
  (UserInterface|Viewport|AddtoViewport _returnvalue 0))

(event Input|ActionEvents|InputActionFire
  (params (Key :type Key%20Structure))
  (:Pressed
    (bind _asbp_cannon (Utilities|Casting|CastToBP_Cannon (Pawn|GetControlledPawn)))
    (Default|Fire _asbp_cannon)))

(event Input|AxisEvents|InputAxisRaiseCannon
  (params (AxisValue :type Float%20%28single-precision%29))
  (if (!= AxisValue 0.0)
    (bind _asbp_cannon (Utilities|Casting|CastToBP_Cannon (Pawn|GetControlledPawn)))
    (Default|RaiseCannon _asbp_cannon AxisValue)))

(fn ConstructionScript)