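; BP_Cannon is a cannon that pitches up and down and fires physics-driven projectiles.
; The RaiseCannon event adds pitch to the Arrow component in proportion to its axis value.
; Fire spawns a BP_Projectile at the Barrel's transform and launches it with a fixed-strength impulse on its Sphere along the Barrel's forward direction.
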(event Custom|Fire
  (bind _barrel (Variables|Default|GetBarrel))
  (bind _returnvalue (Transformation|GetWorldTransform _barrel))
  (bind _returnvalue_2 (Game|SpawnActorfromClass "/Game/AngryTowers/BP_Projectile.BP_Projectile_C" (Math|Transform|MakeTransform (.location _returnvalue) (.rotation _returnvalue) "1,1,1") "Undefined" 0 0))
  (Physics|AddImpulse (Variables|/Game/AngryTowers/BP_Projectile.BP_Projectile_C|GetSphere _returnvalue_2) (Math|Vector|RotateVector (Math|Vector|MakeVector 3e+03 0.0 0.0) (Transformation|GetWorldRotation (Variables|Default|GetBarrel))) "None" false))

(event Custom|RaiseCannon
  (params (Axis%20Value :type Float%20%28single-precision%29))
  (Transformation|AddRelativeRotation (Variables|Default|GetArrow) (Math|Rotator|MakeRotator 0.0 (* Axis%20Value 5.0) 0.0) false false))

(fn ConstructionScript)